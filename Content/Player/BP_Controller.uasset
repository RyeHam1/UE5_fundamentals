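; Player controller that turns input into movement, mouse look, jumping and crouching for player 0's pawn or character.
; Movement axes push the pawn along forward and right vectors built from control yaw only, so camera pitch does not affect direction.
; Jump and crouch start on press and stop on release.
; Punching logic (random montage, grounded check, timed DoOnce, movement locking) exists but is unconnected and never runs.
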(event EventBeginPlay)

(event EventTick
  (params (DeltaSeconds :type Float%20%28single-precision%29)))

(event Input|ActionEvents|InputActionJump
  (params (Key :type Key%20Structure))
  ;[1 1 1] Jumping input
  (:Pressed
    (Character|Jump (Game|GetPlayerCharacter 0)))
  (:Released
    (Character|StopJumping (Game|GetPlayerCharacter 0))))

(event Input|AxisEvents|InputAxisLookUp(mouse)
  (params (AxisValue :type Float%20%28single-precision%29))
  (Pawn|Input|AddControllerPitchInput (Game|Player|GetPlayerPawn 0) AxisValue))

(event Input|AxisEvents|InputAxisTurn(Mouse)
  (params (AxisValue :type Float%20%28single-precision%29))
  (Pawn|Input|AddControllerYawInput (Game|Player|GetPlayerPawn 0) AxisValue))

(event Input|AxisEvents|InputAxisFowardMotion
  (params (AxisValue :type Float%20%28single-precision%29))
  (Pawn|Input|AddMovementInput (Game|Player|GetPlayerPawn 0) (Math|Vector|GetForwardVector (Math|Rotator|MakeRotator 0.0 0.0 (.Yaw (Math|Rotator|BreakRotator (Pawn|GetControlRotation :!class /Script/Engine.Controller))))) AxisValue false))

(event Input|AxisEvents|InputAxisRightMotion
  (params (AxisValue :type Float%20%28single-precision%29))
  (Pawn|Input|AddMovementInput (Game|Player|GetPlayerPawn 0) (Math|Vector|GetRightVector (Math|Rotator|MakeRotator 0.0 0.0 (.Yaw (Math|Rotator|BreakRotator (Pawn|GetControlRotation :!class /Script/Engine.Controller))))) AxisValue false))

(event Input|ActionEvents|InputActionCrouch
  (params (Key :type Key%20Structure :default "None"))
  (:Pressed
    (Character|Crouch (Game|GetPlayerCharacter 0)))
  (:Released
    (Character|UnCrouch (Game|GetPlayerCharacter 0))))

(fn ConstructionScript)