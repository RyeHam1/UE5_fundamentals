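; BP_FIghter is the player fighter character, handling punching, sprinting, a crawl animation on crouch, health and HUD creation.
; Attack plays a random punch montage while grounded, gated by IsPunching and a DoOnce that reset after a short delay.
; Sprint toggles walk speed, and BeginPlay adds the HUD widget.
; AnyDamage reduces Health, and at zero disables input, ragdolls the mesh and detaches the camera in world space.
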(event EventBeginPlay
  (bind _returnvalue (UserInterface|CreateWidget "/Game/WG_HUD.WG_HUD_C"))
  (UserInterface|Viewport|AddtoViewport _returnvalue 0))

(event Input|ActionEvents|InputActionAttack
  (params (Key :type Key%20Structure :default "None"))
  (:Pressed
    (if (and (not (AI|Components|NavMovement|IsFalling (Pawn|GetMovementComponent (Game|GetPlayerCharacter 0)))) (not (Variables|Default|Getis%20Punching)))
      (Variables|Default|Setis%20Punching true)
      (Utilities|FlowControl|DoOnce false :!label _label
        (:Completed
          (Animation|Montage|PlayMontage (Variables|/Script/Engine.Character|GetMesh (Game|GetPlayerCharacter 0)) (Utilities|Array|Get(acopy) (Variables|Default|GetPunch%20Anim%20Array) (Math|Random|RandomIntegerinRange 0 3)) 1.2
            (:then
              (Utilities|FlowControl|Delay 0.5)
              (Variables|Default|Setis%20Punching false)
              (goto _label Reset))))))))

(event Input|ActionEvents|InputActionSprint
  (params (Key :type Key%20Structure :default "None"))
  (:Pressed
    (Variables|/Script/Engine.CharacterMovementComponent|SetMaxWalkSpeed (Variables|Character|GetCharacterMovement) 7e+02))
  (:Released
    (Variables|/Script/Engine.CharacterMovementComponent|SetMaxWalkSpeed (Variables|Character|GetCharacterMovement) 2e+02)))

(event Input|ActionEvents|InputActionCrouch
  (params (Key :type Key%20Structure :default "None"))
  (:Pressed
    (Components|Animation|SetAnimation (Variables|Character|GetMesh) "/Game/Player/Fighter/Animation/Low_Crawl.Low_Crawl")))

(event Game|Damage|EventAnyDamage
  (params (Damage :type Float%20%28single-precision%29) (DamageType :type Damage%20Type%20Object%20Reference) (InstigatedBy :type Controller%20Object%20Reference) (DamageCauser :type Actor%20Object%20Reference))
  (bind _mesh (Variables|Character|GetMesh))
  ;[1 1 1] Take Damage
  (bind _output_get (Variables|Default|SetHealth (- (Variables|Default|GetHealth) Damage)))
  ;[1 1 1] Dies and ragdolls
  (if (<= _output_get 0.0)
    (Input|DisableInput (Game|GetPlayerController 0))
    (Collision|SetCollisionProfileName _mesh "Ragdoll" true :!class /Script/Engine.PrimitiveComponent)
    (Physics|SetSimulatePhysics _mesh true)
    (Transformation|DetachFromComponent (Variables|Default|GetCamera) "KeepWorld" "KeepWorld" "KeepWorld" true)))

(fn ConstructionScript)