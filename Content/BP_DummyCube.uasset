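; BP_DummyCube is a damageable dummy that takes hits from a punching BP_FIghter and drops loot on death.
; Overlapping its Er component while the fighter punches subtracts Damage from Health, with a DoOnce and short delay throttling repeat hits.
; At zero Health it spawns BP_Loot at the mesh transform and destroys itself.
; A separate loot event, not called in this graph, traces downward to spawn BP_Loot at the hit location.
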(event OnComponentBeginOverlap(er)
  (params (OverlappedComponent :type Primitive%20Component%20Object%20Reference) (OtherActor :type Actor%20Object%20Reference) (OtherComp :type Primitive%20Component%20Object%20Reference) (OtherBodyIndex :type Integer) (bFromSweep :type Boolean) (SweepResult :type Hit%20Result%20Structure%20%28by%20ref%29))
  (bind _asbp_fighter (Utilities|Casting|CastToBP_FIghter OtherActor))
  (if (Variables|/Game/Player/Fighter/BP_FIghter.BP_FIghter_C|Getis%20Punching _asbp_fighter)
    (Utilities|FlowControl|DoOnce false :!label _label
      (:Completed
        (Development|PrintString "Hello")
        (bind _output_get (Variables|Default|SetHealth (- (Variables|Default|GetHealth) (Variables|Default|GetDamage))))
        (if (<= _output_get 0)
          (Game|SpawnActorfromClass "/Game/BP_Loot.BP_Loot_C" (Transformation|GetWorldTransform (Variables|Debug|GetStaticMeshComponent)) "Undefined" 0 0)
          (Actor|DestroyActor)
          (Development|PrintString "IM DEAD")
          (else
            (Utilities|FlowControl|Delay 0.2)
            (goto _label Reset)))))))

(event Custom|loot
  (bind _returnvalue (Transformation|GetActorLocation))
  (bind _outhit (Collision|LineTraceByChannel _returnvalue (- _returnvalue "0,0,200.000000") "TraceTypeQuery1" false (Utilities|Array|MakeArray (Game|GetPlayerCharacter 0)) "None"))
  (Game|SpawnActorfromClass "/Game/BP_Loot.BP_Loot_C" (Math|Transform|MakeTransform (.Location (Collision|BreakHitResult _outhit))) "AdjustIfPossibleButDontSpawnIfColliding" 0 0))

(event EventBeginPlay)

(event EventTick
  (params (DeltaSeconds :type Float%20%28single-precision%29)))

(fn ConstructionScript)